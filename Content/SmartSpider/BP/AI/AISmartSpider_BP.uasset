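; Spider character Blueprint that crawls across floors, walls and edges by orienting itself to the surface beneath it.
; Each tick, angled and downward traces classify the surface as plane, concave or convex.
; Planes trigger interpolated sticking at feet offset, concave corners align to the forward hit normal, and convex edges pitch the pawn over.
; Gravity stays off in Flying mode because its check receives a zero normal; BeginPlay adds cables at mesh sockets.
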(event Custom|OnSurfaceCrossDone
  ;[1 1 1] Notity when pawn on crossing surface.
  (Variables|Runtime|SetDisableMovement false))

(event Custom|CrossSurfaceNotify
  ;[1 1 1] Notity when pawn on crossing surface.
  (Variables|Runtime|SetDisableMovement false))

(event Custom|SurfaceChangeNotify
  (params (NewSurface :type SurfaceType%20Enum :default "NewEnumerator0"))
  ;[1 1 1] Notify when pawn cross the surface from one to another.
  (switch Utilities|FlowControl|Switch|SwitchonSurfaceType NewSurface
    (:NewEnumerator0
      _)
    (:NewEnumerator2
      _))
  (Variables|Runtime|SetDisableMovement false)
  (Development|PrintString (Utilities|String|Append (Utilities|String|EnumtoString (Variables|Runtime|GetLastSurfaceType)) (Utilities|String|EnumtoString NewSurface))))

(event EventBeginPlay
  (CallFunction|InitTracingArgs)
  (Class|SkeletalMeshComponent|SetPhysicsBlendWeight (Variables|Character|GetMesh) 0.0)
  (for _array_element (Transformation|GetAllSocketNames (Variables|Character|GetMesh))
    (AddComponent|AddCableComponent false (Transformation|GetSocketTransform (Variables|Character|GetMesh) _array_element "RTS_ParentBoneSpace"))))

(event EventTick
  (params (DeltaSeconds :type Float%20%28single-precision%29))
  (CallFunction|TraceEnv)
  (CallFunction|UpdateRotationRate))

(fn ConstructionScript)

(fn TraceEnv
  (Utilities|FlowControl|Sequence
    (:then_0
      (bind _outhit (Utilities|GetHitResultForward)))
    (:then_1
      (bind _outhit_2 (Utilities|GetHitResultBackward)))
    (:then_2
      (bind _outhit_3 (Utilities|GetHitResultwithBottom)))
    (:then_3
      (bind _surface (Surface|GetSurfaceType _outhit _outhit_2 _outhit_3))
      (bind _outsurfacetype (SurfaceHandle|OnSurfaceHandle _surface _outhit _outhit_2 _outhit_3))
      (Utilities|FireSurfaceEventifChange _outsurfacetype)
      (Variables|Runtime|SetLastSurfaceType _outsurfacetype))
    (:then_4
      (Utilities|EnableGravityifonPlane)
      (if (Variables|Runtime|GetNeedStrickToSurface)
        (Surface|StricktoSurface (Variables|Runtime|GetTransitionSurfaceNormal))))))

(fn GetDrawType
  (if (Variables|Default|GetDebugOn)
    (return "Persistent")
    (else
      (return "None"))))

(fn GetImpactInfo
  (params (Forward :type Acceptable%20Hit%20Result%20Structure) (Backward :type Acceptable%20Hit%20Result%20Structure))
  (bind _hitresult (Utilities|Struct|BreakAcceptableHitResult Forward))
  (bind _hitresult_2 (Utilities|Struct|BreakAcceptableHitResult Backward))
  (bind (_bblockinghit _binitialoverlap _time _distance _location _impactpoint _normal _impactnormal) (Collision|BreakHitResult _hitresult))
  (bind (_bblockinghit_2 _binitialoverlap_2 _time_2 _distance_2 _location_2 _impactpoint_2 _normal_2 _impactnormal_2) (Collision|BreakHitResult _hitresult_2))
  (if _bblockinghit
    (return _impactnormal _impactpoint)
    (elif _bblockinghit_2
      (return _impactnormal_2 _impactpoint_2)
      (else
        (return "0,0.000000,1.000000" "0, 0, 0")))))

(fn TransitiontoSurface
  (params (SurfaceNormal :type Vector) (TransitionPosition :type Vector))
  (bind _returnvalue (Transformation|GetActorRightVector))
  (bind _returnvalue_2 (Math|Vector|CrossProduct _returnvalue SurfaceNormal))
  (Transformation|SetActorTransform (Math|Transform|MakeTransform TransitionPosition (Math|Rotator|MakeRotationfromAxes _returnvalue_2 (Math|Vector|CrossProduct SurfaceNormal _returnvalue_2) SurfaceNormal) (Transformation|GetActorScale3D)) false true))

(fn StricktoSurface
  (params (SurfaceNormal :type Vector))
  (bind _returnvalue (Transformation|GetActorUpVector))
  (bind _returnvalue_2 (Utilities|Time|GetWorldDeltaSeconds))
  (bind _returnvalue_3 (Math|Interpolation|VInterpTo _returnvalue SurfaceNormal _returnvalue_2 5e+01))
  (bind (_outhit _returnvalue_4) (CallFunction|GetHitwithLocation self (Transformation|GetActorLocation) (- "0, 0, 0" (Transformation|GetActorUpVector)) (Variables|EnvironmentTracing|Distance|GetStrickDetectDistance) (Variables|Default|GetDebugOn) (Variables|EnvironmentTracing|Rays|GetTraceColor_Center)))
  (if _returnvalue_4
    (bind _isalign (Utilities|IsAlignwithSurface (.ImpactPoint (Collision|BreakHitResult _outhit))))
    (if (not _isalign)
      (Surface|TransitiontoSurface _returnvalue_3 (CallFunction|CalcDesireStrickLocation (.ImpactPoint (Collision|BreakHitResult _outhit)) _returnvalue_3)))))

(fn CalcDesireStrickLocation
  (params (ImpactPoint :type Vector) (SurfaceNormal :type Vector))
  (bind _offset (CallFunction|GetPawnFeetOffset self))
  (return (+ (* SurfaceNormal _offset) ImpactPoint)))

(fn OnPlaneHandle
  (params (HitResultForward :type Acceptable%20Hit%20Result%20Structure) (HitResultBackward :type Acceptable%20Hit%20Result%20Structure) (HitResultBottom :type Acceptable%20Hit%20Result%20Structure))
  (bind _hitresult (Utilities|Struct|BreakAcceptableHitResult HitResultBottom))
  (bind (_bblockinghit _binitialoverlap _time _distance _location _impactpoint _normal _impactnormal) (Collision|BreakHitResult _hitresult))
  (if _bblockinghit
    (return true _impactnormal)
    (else
      (return true (Transformation|GetActorUpVector)))))

(fn OnConvexHandle
  (params (HitResultForward :type Acceptable%20Hit%20Result%20Structure) (HitResultBackward :type Acceptable%20Hit%20Result%20Structure) (HitResultBottom :type Acceptable%20Hit%20Result%20Structure))
  ;[1 1 1] When cross the surface, only rotate along pitch is allowed and movement ability should disable to make transition smooth.
  (CallFunction|CrossSurfaceNotify)
  (Transformation|AddActorLocalRotation (Class|KismetMathLibrary|NegateRotator (Math|Rotator|MakeRotator 0.0 (* (Variables|EnvironmentTracing|GetRotationSpeed) (Utilities|Time|GetWorldDeltaSeconds)) 0.0)) false true)
  (return false "0, 0, 0"))

(fn OnConcaveHandle
  (params (HitResultForward :type Acceptable%20Hit%20Result%20Structure) (HitResultBackward :type Acceptable%20Hit%20Result%20Structure) (HitResultBottom :type Acceptable%20Hit%20Result%20Structure))
  (Surface|TransitiontoSurface (.ImpactNormal (Collision|BreakHitResult (.HitResult (Utilities|Struct|BreakAcceptableHitResult HitResultForward)))) (Transformation|GetActorLocation))
  (return false "0, 0, 0"))

(fn InitTracingArgs
  (bind _returnvalue (Utilities|CalcSurfaceTracingDistance))
  (Variables|Runtime|SetAcceptableSurfaceTraceingDistanceSq (* _returnvalue _returnvalue))
  (bind _offset (CallFunction|GetPawnFeetOffset self))
  (Variables|Runtime|SetAcceptableTransitionDetectDistanceSq (* _offset _offset)))

(fn SurfaceAcceptableTest
  (params (HitResult :type Hit%20Result%20Structure))
  (return (and (.bBlockingHit (Collision|BreakHitResult HitResult)) false)))

(fn OnSurfaceHandle
  (params (SurfaceType :type SurfaceType%20Enum :default "NewEnumerator0") (HitResultForward :type Acceptable%20Hit%20Result%20Structure) (HitResultBackward :type Acceptable%20Hit%20Result%20Structure) (HitResultBottom :type Acceptable%20Hit%20Result%20Structure))
  (switch Utilities|FlowControl|Switch|SwitchonSurfaceType SurfaceType
    (:NewEnumerator0
      (bind (_needstricktosurface _transitionsurfacenormal) (SurfaceHandle|OnPlaneHandle HitResultForward HitResultBackward HitResultBottom))
      (Variables|Runtime|SetNeedStrickToSurface _needstricktosurface)
      (Variables|Runtime|SetTransitionSurfaceNormal _transitionsurfacenormal))
    (:NewEnumerator1
      (bind _needstricktosurface_2 (SurfaceHandle|OnConvexHandle HitResultForward HitResultBackward HitResultBottom))
      (Variables|Runtime|SetNeedStrickToSurface _needstricktosurface_2))
    (:NewEnumerator2
      (bind _transitionsurfacenormal_2 (SurfaceHandle|OnConcaveHandle HitResultForward HitResultBackward HitResultBottom))
      (Variables|Runtime|SetTransitionSurfaceNormal _transitionsurfacenormal_2)))
  (return SurfaceType))

(fn GetSurfaceType
  (params (HitResultForward :type Acceptable%20Hit%20Result%20Structure) (HitResultBackward :type Acceptable%20Hit%20Result%20Structure) (HitResultBottom :type Acceptable%20Hit%20Result%20Structure))
  (bind _isconcave (Surface|IsSurfaceConcave HitResultForward HitResultBackward HitResultBottom))
  (if _isconcave
    (return "NewEnumerator2")
    (else
      (bind _isplane (Surface|IsSurfacePlane HitResultForward HitResultBackward HitResultBottom))
      (if _isplane
        (return "NewEnumerator0")
        (else
          (return "NewEnumerator1"))))))

(fn UpdateRotationRate
  (bind _returnvalue (Math|Rotator|MakeRotator 0.0 3.6e+02 0.0))
  (bind _returnvalue_2 (Transformation|GetActorTransform))
  (bind (_x _y _z) (Math|Rotator|BreakRotIntoAxes _returnvalue))
  (Variables|/Script/Engine.CharacterMovementComponent|SetRotationRate (Variables|Character|GetCharacterMovement) (Math|Rotator|MakeRotationfromAxes (Math|Transform|TransformLocation _returnvalue_2 _x) (Math|Transform|TransformLocation _returnvalue_2 _y) (Math|Transform|TransformLocation _returnvalue_2 _z))))

(fn DistanceTestAgainst
  (params (Hit :type Hit%20Result%20Structure%20%28by%20ref%29) (TestDistanceSq :type Float%20%28single-precision%29) (TestTolerance :type Float%20%28single-precision%29))
  (bind (_bblockinghit _binitialoverlap _time _distance _location _impactpoint _normal _impactnormal _physmat _hitactor _hitcomponent _hitbonename _hititem _faceindex _tracestart) (Collision|BreakHitResult Hit))
  (if _bblockinghit
    (Utilities|DistanceTest _tracestart _impactpoint TestDistanceSq TestTolerance
      (:Equal
        (return (Utilities|Struct|MakeAcceptableHitResult true "NewEnumerator0" Hit TestDistanceSq TestTolerance)))
      (:GreaterThan
        (return (Utilities|Struct|MakeAcceptableHitResult false "NewEnumerator1" Hit TestDistanceSq TestTolerance)))
      (:LessThan
        (return (Utilities|Struct|MakeAcceptableHitResult false "NewEnumerator2" Hit TestDistanceSq TestTolerance))))
    (else
      ;[1 1 1] Hits nothing means tracing distance greater than the desire test against distance
      (return (Utilities|Struct|MakeAcceptableHitResult false "NewEnumerator1" Hit)))))

(fn IsSurfacePlane
  (params (HitResultForward :type Acceptable%20Hit%20Result%20Structure) (HitResultBackward :type Acceptable%20Hit%20Result%20Structure) (HitResultBottom :type Acceptable%20Hit%20Result%20Structure))
  (bind _hitresult (Utilities|Struct|BreakAcceptableHitResult HitResultBottom))
  (bind (_bblockinghit _binitialoverlap _time _distance _location _impactpoint _normal _impactnormal) (Collision|BreakHitResult _hitresult))
  (bind _outhit (Utilities|GetHitResultwithBottomAssistor))
  (return (Math|Boolean|ANDBoolean (.bBlockingHit (Collision|BreakHitResult (.HitResult (Utilities|Struct|BreakAcceptableHitResult _outhit)))) _bblockinghit (Math|Vector|Equal(Vector) (.ImpactNormal (Collision|BreakHitResult (.HitResult (Utilities|Struct|BreakAcceptableHitResult _outhit)))) _impactnormal 0.01))))

(fn IsSurfaceConcave
  (params (HitResultForward :type Acceptable%20Hit%20Result%20Structure) (HitResultBackward :type Acceptable%20Hit%20Result%20Structure) (HitResultBottom :type Acceptable%20Hit%20Result%20Structure))
  (return (Utilities|Enum|Equal(Enum) (.DistanceTestResult (Utilities|Struct|BreakAcceptableHitResult HitResultForward)) "NewEnumerator2")))

(fn Moveto
  (params (Location :type Vector))
  (Pawn|Input|AddMovementInput (Math|Vector|Normalize (- Location (Transformation|GetActorLocation))) 1.0 false)
  (return false))